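; RPG HUD Blueprint that shows the player's on-screen HUD and item pickup notifications.
; BeginPlay creates WBP_HUD and adds it to the viewport.
; PushNewItemNotification creates a WBP_ItemAdded entry for the item, adds it to the HUD's vertical box, and plays the Notch animation and a sound.
; XP, health, stamina and adrenaline update events are empty, with their SetPercent calls left disconnected.
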(event `self.ReceiveBeginPlay`
  ;[0 0 0 0.5] ゲーム開始時にＨＵＤ表示
  (bind _returnvalue (`|CreateWidget` "/Game/BluePrint/UI/WBP_HUD.WBP_HUD_C" (`GameplayStatics.GetPlayerController` 0)))
  (bind _output_get (set `self.HUD` _returnvalue))
  (`UserWidget.AddToViewport` _output_get 0))

(event `/Game/BluePrint/UI/BPI_RPG_HUD.UpdateXPBar`
  (params (NewPercentage :type "Float (double-precision)"))
  ;[0 0 0 0.5] ゲーム開始時にＨＵＤ表示
)

(event `/Game/BluePrint/UI/BPI_RPG_HUD.UpdateStaminaBar`
  (params (NewPercentage :type "Float (double-precision)"))
  ;[0 0 0 0.5] ゲーム開始時にＨＵＤ表示
)

(event `/Game/BluePrint/UI/BPI_RPG_HUD.UpdateHealthBar`
  (params (NewPercentage :type "Float (double-precision)"))
  ;[0 0 0 0.5] ゲーム開始時にＨＵＤ表示
)

(event `/Game/BluePrint/UI/BPI_RPG_HUD.UpdateAdrenalineBar`
  (params (NewPercentage :type "Float (double-precision)"))
  ;[0 0 0 0.5] ゲーム開始時にＨＵＤ表示
)

(event `/Game/Menu/UI/BPI_InventoryHUD.PushNewItemNotification`
  (params (Item :type "RPGItem Structure"))
  (bind _hud (`self.HUD`))
  ;[0 0 0 0.5] インタラクト成功
  ;;[0 0 0 0.5] アイテムインタラクト時に入手ウィジェットの表示
  (bind _returnvalue (`|CreateWidget` "/Game/Menu/UI/WBP_ItemAdded.WBP_ItemAdded_C" null Item))
  (`UserWidget.PlayAnimation` _hud (`/Game/BluePrint/UI/WBP_HUD.Notch` _hud) 0.0 1 "Forward" 1.0 false)
  (`VerticalBox.AddChildToVerticalBox` (`/Game/BluePrint/UI/WBP_HUD.VerticalBox_183` (`self.HUD`)) _returnvalue)
  (`GameplayStatics.PlaySound2D` "/Game/Audio/SE/text-notification-96707.text-notification-96707" 1.0 1.0 0.0 null null))

(fn `UserConstructionScript`)