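; RPG player controller that opens and closes the in-game menu from Enhanced Input actions.
; Opening creates the game mode's menu widget with the requested tab, pauses, shows the cursor and adds the menu mapping context; closing reverses this.
; Menu and Note actions share one FlipFlop, opening the same tab.
; Item and Map actions are empty, with two disconnected FlipFlops left in the graph.
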(event `self.ReceiveBeginPlay`)

(event `/Game/BluePrint/Interface/BPI_RPGPlayerController.OpenGameMenu`
  (params (ActiveMenu :type "/Game/Inputs/GameMenu/E_GameMenus Enum" :default "NewEnumerator0"))
  (bind _gamemodeclass (message `/Game/BluePrint/Interface/BPI_RPGGameMode.GetGameMenuClass` (`GameplayStatics.GetGameMode`)))
  (bind _returnvalue (`|CreateWidget` _gamemodeclass self))
  (bind _output_get (set `self.InGameMenu` _returnvalue))
  (message `/Game/Inputs/GameMenu/BPI_GameMenu.SetActiveMenu` _output_get ActiveMenu)
  (`UserWidget.AddToViewport` (`self.InGameMenu`) 0)
  (`WidgetBlueprintLibrary.SetInputMode_GameAndUIEx` self (`self.InGameMenu`))
  (set `self.bShowMouseCursor` true)
  (`GameplayStatics.SetGamePaused` true)
  (`EnhancedInputSubsystemInterface.AddMappingContext` (pcsubsystem `EnhancedInputLocalPlayerSubsystem` self) "/Game/Inputs/IMC_InGameMenu.IMC_InGameMenu" 1 (struct)))

(event `/Game/BluePrint/Interface/BPI_RPGPlayerController.CloseGameMenu`
  (`Widget.RemoveFromParent` (`self.InGameMenu`))
  (set `self.InGameMenu` null)
  (`WidgetBlueprintLibrary.SetInputMode_GameOnly` self)
  (set `self.bShowMouseCursor` false)
  (`GameplayStatics.SetGamePaused` false)
  (`EnhancedInputSubsystemInterface.RemoveMappingContext` (pcsubsystem `EnhancedInputLocalPlayerSubsystem` self) "/Game/Inputs/IMC_InGameMenu.IMC_InGameMenu" (struct)))

(event `EnhancedInput|/Game/Inputs/Actions/IA_ToggleMenu`
  (params (ActionValue :type Boolean) (ElapsedSeconds :type "Float (double-precision)") (TriggeredSeconds :type "Float (double-precision)") (InputAction :type "InputAction Object Reference" :default "/Game/Inputs/Actions/IA_ToggleMenu.IA_ToggleMenu"))
  (:`Started`
    (`/Engine/EditorBlueprintResources/StandardMacros.FlipFlop` :!label _label
      (:`A`
        (`self.OpenGameMenu` "NewEnumerator3"))
      (:`B`
        (`self.CloseGameMenu`)))))

(event `EnhancedInput|/Game/Inputs/Actions/IA_ToggleNote`
  (params (ActionValue :type Boolean) (ElapsedSeconds :type "Float (double-precision)") (TriggeredSeconds :type "Float (double-precision)") (InputAction :type "InputAction Object Reference" :default "/Game/Inputs/Actions/IA_ToggleNote.IA_ToggleNote"))
  (:`Started`
    (goto _label)))

(event `EnhancedInput|/Game/Inputs/Actions/IA_ToggleItem`
  (params (ActionValue :type Boolean) (ElapsedSeconds :type "Float (double-precision)") (TriggeredSeconds :type "Float (double-precision)") (InputAction :type "InputAction Object Reference" :default "/Game/Inputs/Actions/IA_ToggleItem.IA_ToggleItem")))

(event `EnhancedInput|/Game/Inputs/Actions/IA_ToggleMap`
  (params (ActionValue :type Boolean) (ElapsedSeconds :type "Float (double-precision)") (TriggeredSeconds :type "Float (double-precision)") (InputAction :type "InputAction Object Reference" :default "/Game/Inputs/Actions/IA_ToggleMap.IA_ToggleMap")))

(fn `UserConstructionScript`)