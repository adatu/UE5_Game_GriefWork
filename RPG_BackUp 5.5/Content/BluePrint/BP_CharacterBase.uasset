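; BP_CharacterBase is a character base Blueprint that exposes the character's vital stats and progression as ratios.
; Four functions compute health, stamina, adrenaline and experience point percentages, each dividing the current getter value by its maximum getter value without clamping or zero checks.
; The event graph and construction script hold no logic.
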(fn `GetAdrenalinePercentage`
  (returns (ReturnValue :type "Float (double-precision)"))
  (return (/ (`self.GetAdrenaline`) (`self.GetMaxAdrenaline`))))

(fn `GetHealthPercentage`
  (returns (ReturnValue :type "Float (double-precision)"))
  (return (/ (`self.GetHealth`) (`self.GetMaxHealth`))))

(fn `GetStaminaPercentage`
  (returns (ReturnValue :type "Float (double-precision)"))
  (return (/ (`self.GetStamina`) (`self.GetMaxStamina`))))

(fn `GetXPPercentage`
  (returns (ReturnValue :type "Float (double-precision)"))
  (return (/ (`self.GetExperiencePoints`) (`self.GetMaxExperiencePoints`))))

(fn `UserConstructionScript`)