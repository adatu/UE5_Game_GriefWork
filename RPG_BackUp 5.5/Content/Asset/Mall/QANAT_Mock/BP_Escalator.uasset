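; Escalator actor that moves a continuous loop of step meshes along a spline, forward or reversed.
; The construction script fills StepArray with static mesh components spaced by StepOffset along the spline length.
; Tick advances one shared distance at constant speed, offsets each step by its index and wraps it at the spline's end.
; Only step locations follow the spline, not rotations, and the shared distance resets on reaching either end.
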(event `self.ReceiveTick`
  (params (DeltaSeconds :type "Float (single-precision)"))
  (bind _returnvalue (`SplineComponent.GetSplineLength` (`self.Spline`)))
  (if (`KismetArrayLibrary.Array_IsValidIndex` (`self.StepArray`))
    (set `self.DistanceAlongSprine` (`KismetMathLibrary.FInterpTo_Constant` (`self.DistanceAlongSprine`) (`KismetMathLibrary.SelectFloat` 0.0 (`SplineComponent.GetSplineLength` (`self.Spline`)) (`self.Reverse?`)) (`GameplayStatics.GetWorldDeltaSeconds`) (`self.IniterSpeed`)))
    (for (_array_element _array_index) (`self.StepArray`)
      (bind _returnvalue_2 (+ (`self.DistanceAlongSprine`) (* _array_index (`self.StepOffset`))))
      (`SceneComponent.K2_SetWorldLocation` _array_element (`SplineComponent.GetLocationAtDistanceAlongSpline` (`self.Spline`) (`KismetMathLibrary.SelectFloat` (- _returnvalue_2 _returnvalue) _returnvalue_2 (> _returnvalue_2 _returnvalue)) "World") false false))
    (if (`KismetMathLibrary.NearlyEqual_FloatFloat` (`self.DistanceAlongSprine`) (`KismetMathLibrary.SelectFloat` 0.0 (`SplineComponent.GetSplineLength` (`self.Spline`)) (`self.Reverse?`)))
      (set `self.DistanceAlongSprine` (`KismetMathLibrary.SelectFloat` (`SplineComponent.GetSplineLength` (`self.Spline`)) 0.0 (`self.Reverse?`))))))

(fn `UserConstructionScript`
  (`KismetArrayLibrary.Array_Clear` (`self.StepArray`))
  (for _index (range (+ (`KismetMathLibrary.FFloor` (/ (`SplineComponent.GetSplineLength` (`self.Spline`)) (`self.StepOffset`))) 1))
    (bind _returnvalue (`AddComponent|NODE_AddStaticMeshComponent-0` :`RelativeTransform` (`KismetMathLibrary.MakeTransform` (`SplineComponent.GetLocationAtDistanceAlongSpline` (`self.Spline`) (* _index (`self.StepOffset`)) "Local"))))
    (`KismetArrayLibrary.Array_Add` (`self.StepArray`) _returnvalue)))